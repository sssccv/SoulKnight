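; Boss enemy Blueprint that shows a boss health bar on screen when the player character enters its trigger.
; On BossTrigger overlap with BP_ThirdPersonCharacter, it creates a WB_BossHealth widget and adds it to the viewport.
; After a one-tick delay, it passes the widget's progress bar to BPCStats via SetHealthProgressBar.
; The overlap has no once-only guard, so each re-entry creates another widget.
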(event `self.BossTrigger.OnComponentBeginOverlap`
  (params (OverlappedComponent :type "PrimitiveComponent Object Reference") (OtherActor :type "Actor Object Reference") (OtherComp :type "PrimitiveComponent Object Reference") (OtherBodyIndex :type Integer) (bFromSweep :type Boolean) (SweepResult :type "HitResult Structure (by ref)"))
  (cast `/Game/ThirdPerson/Blueprints/BP_ThirdPersonCharacter` OtherActor)
  (bind _returnvalue (`|CreateWidget` "/Game/UI/WB_BossHealth.WB_BossHealth_C"))
  (bind _output_get (set `self.BossHealthWidget` _returnvalue))
  (`UserWidget.AddToViewport` _output_get 0)
  (`KismetSystemLibrary.DelayUntilNextTick`)
  (`/Game/Blueprints/BPC_Stats.Set Health Progress Bar` (`self.BPC_Stats`) (`/Game/UI/WB_BossHealth.hEALTHbAR` (`self.BossHealthWidget`))))

(fn `UserConstructionScript`
  (`parent.UserConstructionScript`))