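; Player combat component for BP_ThirdPersonCharacter, handling target lock, sword combos, hit detection and dodge rolls.
; Lock-on sphere-traces from the camera, spawns a marker on the target and steers control rotation toward it each Tick.
; One attack montage continues past each notify only if another press was queued.
; A looping timer sweeps between sword points with throttled damage, while dodges pick directional rolls from WASD when strafing.
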(event `self.ReceiveBeginPlay`
  ; GetPlayerClass
  (bind _asbp_third_person_character (cast `/Game/ThirdPerson/Blueprints/BP_ThirdPersonCharacter` (`self.GetOwner`)))
  (set `self.playerBP` _asbp_third_person_character))

(event `EnhancedInput|/Game/ThirdPerson/Input/Actions/IA_Lock`
  (params (ActionValue :type Boolean) (ElapsedSeconds :type "Float (double-precision)") (TriggeredSeconds :type "Float (double-precision)") (InputAction :type "InputAction Object Reference" :default "/Game/ThirdPerson/Input/Actions/IA_Lock.IA_Lock"))
  (bind _returnvalue (`Actor.GetTransform` (`self.TargetLockActor`)))
  (bind _transformcomponent (`PlayerCameraManager.TransformComponent` (`GameplayStatics.GetPlayerCameraManager` 0)))
  (bind _charactermovement (`Character.CharacterMovement` (`self.playerBP`)))
  (bind _charactermovement_2 (`Character.CharacterMovement` (`self.playerBP`)))
  (bind (_returnvalue_x _returnvalue_y _returnvalue_z) (`KismetMathLibrary.BreakVector` (`SceneComponent.K2_GetComponentLocation` _transformcomponent)))
  (bind _returnvalue_2 (`KismetMathLibrary.MakeVector` _returnvalue_x _returnvalue_y (+ _returnvalue_z 20.0)))
  ; TargetLock
  (:`Started`
    (`self.TargetLockActor`
      (:`then`
        (set `self.TargetLockActor` null)
        (set `CharacterMovementComponent.bOrientRotationToMovement` true _charactermovement)
        (set `CharacterMovementComponent.bUseControllerDesiredRotation` false _charactermovement)
        (`Actor.K2_DestroyActor` (`self.TargetLockWidget`)))
      (:`else`
        (bind (_outhit _returnvalue_3) (`KismetSystemLibrary.SphereTraceSingleForObjects` :`Start` _returnvalue_2 :`End` (+ _returnvalue_2 (* (`KismetMathLibrary.GetForwardVector` (`SceneComponent.K2_GetComponentRotation` _transformcomponent)) 1000.0)) :`Radius` 150.0 :`ObjectTypes` (`|MakeArray` "ObjectTypeQuery3" :!type "EObjectTypeQuery Enum") :`DrawTime` 2.0))
        (if _returnvalue_3
          (set `self.TargetLockActor` (`.HitActor` (`GameplayStatics.BreakHitResult` _outhit)))
          (set `CharacterMovementComponent.bOrientRotationToMovement` false _charactermovement_2)
          (set `CharacterMovementComponent.bUseControllerDesiredRotation` true _charactermovement_2)
          (bind _returnvalue_4 (`|SpawnActorFromClass` "/Game/Blueprints/BP_TargetLockWidget.BP_TargetLockWidget_C" (`KismetMathLibrary.MakeTransform` (`KismetMathLibrary.MakeVector` (.x (.location _returnvalue)) (.y (.location _returnvalue)) (+ (.z (.location _returnvalue)) 100.0)) (.rotation _returnvalue)) "AlwaysSpawn" "MultiplyWithRoot" null null))
          (bind _output_get (set `self.TargetLockWidget` _returnvalue_4))
          (`Actor.K2_AttachToActor` _output_get (`self.TargetLockActor`) "None" "SnapToTarget" "SnapToTarget" "SnapToTarget" true))))))

(event `self.ReceiveTick`
  (params (DeltaSeconds :type "Float (single-precision)"))
  (bind (_returnvalue_roll _returnvalue_pitch _returnvalue_yaw) (`KismetMathLibrary.BreakRotator` (`KismetMathLibrary.FindLookAtRotation` (`Actor.K2_GetActorLocation` (`self.playerBP`)) (`Actor.K2_GetActorLocation` (`self.TargetLockActor`)))))
  ; TargetLockUpdate
  (`self.TargetLockActor`
    (:`then`
      (`Controller.SetControlRotation` (`Pawn.GetController` (`self.playerBP`)) (`KismetMathLibrary.MakeRotator` _returnvalue_roll (+ _returnvalue_pitch -20.0) _returnvalue_yaw)))
    (:`else`)))

(event `EnhancedInput|/Game/ThirdPerson/Input/Actions/IA_Attack`
  (params (ActionValue :type Boolean) (ElapsedSeconds :type "Float (double-precision)") (TriggeredSeconds :type "Float (double-precision)") (InputAction :type "InputAction Object Reference" :default "/Game/ThirdPerson/Input/Actions/IA_Attack.IA_Attack"))
  ; SwordComboAnimation
  (:`Started`
    (if (not (`self.isAttacking?`))
      (set `self.isAttacking?` true)
      (`|PlayMontage` (`Character.Mesh` (`self.playerBP`)) "/Game/Characters/Souls/Combat/Sw_MainAttacks_Montage.Sw_MainAttacks_Montage"
        (:`OnCompleted`
          (set `self.isAttacking?` false :!label _label)
          (set `self.combo?` false))
        (:`OnInterrupted`
          (goto _label))
        (:`OnNotifyBegin`
          (if (and (`self.isAttacking?`) (`self.combo?`))
            (set `self.combo?` false)
            (else
              (`AnimInstance.Montage_Stop` (`SkeletalMeshComponent.GetAnimInstance` (`Character.Mesh` (`self.playerBP`))) 0.2 "/Game/Characters/Souls/Combat/Sw_MainAttacks_Montage.Sw_MainAttacks_Montage")))))
      (else
        (set `self.combo?` true)))))

(event `End Damage Trace`
  ; Sword Traces
  (if (`KismetSystemLibrary.K2_IsValidTimerHandle` (stale `Begin Damage Trace` _returnvalue))
    (`KismetSystemLibrary.K2_ClearAndInvalidateTimerHandle` (stale `Begin Damage Trace` _returnvalue))))

(event `Begin Damage Trace`
  ; Sword Traces
  (bind _returnvalue (`KismetSystemLibrary.K2_SetTimerDelegate` (delegate `Damage Trace`) 0.01 true)))

(event `Damage Trace`
  (bind _playerbp (`self.playerBP`))
  ; Sword Traces
  (bind (_outhit _returnvalue) (`KismetSystemLibrary.SphereTraceSingleForObjects` (`SceneComponent.K2_GetComponentLocation` (`/Game/ThirdPerson/Blueprints/BP_ThirdPersonCharacter.Start Sword Trace Pos` _playerbp)) (`SceneComponent.K2_GetComponentLocation` (`/Game/ThirdPerson/Blueprints/BP_ThirdPersonCharacter.End Sword Trace Pos` _playerbp)) 25.0 (`|MakeArray` "ObjectTypeQuery3" :!type "EObjectTypeQuery Enum")))
  (if _returnvalue
    (`/Engine/EditorBlueprintResources/StandardMacros.DoOnce` false :!label _label_2
      (:`Completed`
        (`GameplayStatics.ApplyDamage` (`.HitActor` (`GameplayStatics.BreakHitResult` _outhit)) (`self.Sword Damage`))
        (`KismetSystemLibrary.Delay` 0.5)
        (goto _label_2 :!via `Reset`)))))

(event `EnhancedInput|/Game/ThirdPerson/Input/Actions/IA_Dodge`
  (params (ActionValue :type Boolean) (ElapsedSeconds :type "Float (double-precision)") (TriggeredSeconds :type "Float (double-precision)") (InputAction :type "InputAction Object Reference" :default "/Game/ThirdPerson/Input/Actions/IA_Dodge.IA_Dodge"))
  (:`Started`
    (if (not (`self.IsDodging?`))
      (set `self.IsDodging?` true)
      (`|ExecutionSequence`
        (:`then_0`
          (if (`CharacterMovementComponent.bUseControllerDesiredRotation` (`Character.CharacterMovement` (`self.playerBP`)))
            (switch `string` (`KismetTextLibrary.Conv_TextToString` (`KismetInputLibrary.Key_GetDisplayName` (`/Game/ThirdPerson/Blueprints/BP_ThirdPersonCharacter.Direction Key` (`self.playerBP`))))
              (:`W`
                (set `self.MovementDirection` "NewEnumerator0"))
              (:`A`
                (set `self.MovementDirection` "NewEnumerator2"))
              (:`S`
                (set `self.MovementDirection` "NewEnumerator3"))
              (:`D`
                (set `self.MovementDirection` "NewEnumerator4")))
            (else
              (set `self.MovementDirection` "NewEnumerator0"))))
        (:`then_1`
          (`|PlayMontage` (`Character.Mesh` (`self.playerBP`)) (select `/Game/Blueprints/E_MovementDirection` (`self.MovementDirection`) :`NewEnumerator0` "/Game/SwordAnimationPack/Animations/Roll/Roll_F_Montage.Roll_F_Montage" :`NewEnumerator2` "/Game/Characters/Souls/Combat/Dodge/roll/Sw_RollL_Montage.Sw_RollL_Montage" :`NewEnumerator3` "/Game/Characters/Souls/Combat/Dodge/roll/Sw_RollB_Montage.Sw_RollB_Montage" :`NewEnumerator4` "/Game/Characters/Souls/Combat/Dodge/roll/Sw_RollR_Montage.Sw_RollR_Montage" :!type "AnimMontage Object Reference")
            (:`OnCompleted`
              _)
            (:`OnInterrupted`
              _))
          (set `self.IsDodging?` false))))))